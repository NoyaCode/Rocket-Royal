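; Game mode for Rocket Royal that sets up local split-screen players and their teams when play begins.
; With split-screen toggled off, it creates a player per persistent game instance count, spawning and possessing a military character at the first PlayerStart found.
; It registers characters in the game instance, re-enables split-screen, then assigns teams, applies player meshes and updates team sizes.
; Short delays are placed around player creation.
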(event EventBeginPlay
  (bind _asbp_persistent_game_instance (Utilities|Casting|CastToBP_PersistentGameInstance (Game|GetGameInstance)))
  (Class|PersistentGameInstance|PrintTeamCharacters _asbp_persistent_game_instance)
  (bind _output_get (Variables|Default|SetGameInstance _asbp_persistent_game_instance))
  (Utilities|Array|Clear (Variables|/Script/RocketRoyal.PersistentGameInstance|GetMilitaryCharacters _output_get))
  (Class|RocketRoyalGameModeBase|StartSplitScreen false)
  (Utilities|FlowControl|Delay 0.05)
  (for _index (range 0 (- (Variables|/Script/RocketRoyal.PersistentGameInstance|GetnbPlayers _asbp_persistent_game_instance) 1))
    (Class|GameplayStatics|CreatePlayer _index false)
    (bind _outactors (Actor|GetAllActorsOfClass "/Script/Engine.PlayerStart"))
    (bind _returnvalue (Game|SpawnActorfromClass "/Game/Blueprints/Player/BP_MilitaryCharacter.BP_MilitaryCharacter_C" (Transformation|GetActorTransform (Utilities|Array|Get(acopy) _outactors)) "Undefined" 0 0 0))
    (Pawn|Possess (Game|GetPlayerController _index) _returnvalue)
    (Utilities|Array|AddUnique (Variables|/Script/RocketRoyal.PersistentGameInstance|GetMilitaryCharacters (Variables|Default|GetGameInstance)) _returnvalue)
    (Input|SetInputModeGameOnly (Game|GetPlayerController _index))
    (Utilities|FlowControl|Delay 0.05))
  (Class|RocketRoyalGameModeBase|StartSplitScreen true)
  (Class|PersistentGameInstance|SetTeamsforCharacters (Variables|Default|GetGameInstance))
  (for _array_element (Variables|/Script/RocketRoyal.PersistentGameInstance|GetMilitaryCharacters (Variables|Default|GetGameInstance))
    (Class|MilitaryCharacter|SetMeshPlayer _array_element))
  (Class|PersistentGameInstance|UpdateSizeTeams (Variables|Default|GetGameInstance) false))

(fn ConstructionScript)