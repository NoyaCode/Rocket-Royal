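; Lobby game mode for local multiplayer that shows the lobby widget and sets up player slots at level start.
; Each PlayerStart tag is read as a player index; matching starts get a created local player possessing a spawned BP_InputReceiver.
; SpawnPlayer spawns a BP_LobbyCharacter at a receiver's transform, possesses it, registers it in the persistent game instance and creates its team selector.
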(event EventBeginPlay
  (bind _returnvalue (UserInterface|CreateWidget "/Game/Blueprints/Lobby/BP_LobbyWidget.BP_LobbyWidget_C"))
  (UserInterface|Viewport|AddtoViewport _returnvalue 0)
  (Variables|Default|SetLobbyWidget _returnvalue)
  (CallFunction|GetPlayerStartPoint)
  (CallFunction|SpawnPlayerReceivers))

(fn ConstructionScript)

(fn GetPlayerStartPoint
  (bind _outactors (Actor|GetAllActorsOfClass "/Script/Engine.PlayerStart"))
  (Variables|Default|SetPlayerStart%20Array _outactors))

(fn SpawnPlayerReceivers
  (params (PlayerStart :type Player%20Start%20Object%20Reference))
  (bind _playerstart_array (Variables|Default|GetPlayerStart%20Array))
  (for (_ _array_index) _playerstart_array
    (LocalVariables|SetIndex _array_index)
    (for _array_element _playerstart_array
      (if (== (CallFunction|NametoInt _array_element) (LocalVariables|GetIndex))
        (Class|GameplayStatics|CreatePlayer -1)
        (bind _returnvalue (Game|SpawnActorfromClass "/Game/Blueprints/Lobby/BP_InputReceiver.BP_InputReceiver_C" (Transformation|GetActorTransform _array_element) "Undefined" 0 (LocalVariables|GetIndex) 0))
        (Utilities|Array|AddUnique (Variables|Default|GetPlayerInputReceiverArray) _returnvalue)
        (Pawn|Possess (Game|GetPlayerController (LocalVariables|GetIndex)) _returnvalue)
        (Utilities|Array|AddUnique (Variables|Default|GetPlayerControllerArray) (Game|GetPlayerController (LocalVariables|GetIndex)))))))

(fn NametoInt
  (params (self2 :type Player%20Start%20Object%20Reference))
  (return (Math|Conversions|ToInteger(Byte) (Utilities|String|ToString(Name) (Variables|/Script/Engine.PlayerStart|GetPlayerStartTag self2)))))

(fn SpawnPlayer
  (params (CurrentPlayerIndex :type Integer) (InputReceiver :type BP%20Input%20Receiver%20Object%20Reference))
  (bind _returnvalue (Game|SpawnActorfromClass "/Game/Blueprints/Lobby/BP_LobbyCharacter.BP_LobbyCharacter_C" (Transformation|GetActorTransform InputReceiver) "Undefined" 0 CurrentPlayerIndex 0))
  (Pawn|Possess (Game|GetPlayerController CurrentPlayerIndex) _returnvalue)
  (bind _asbp_persistent_game_instance (Utilities|Casting|CastToBP_PersistentGameInstance (Game|GetGameInstance)))
  (Utilities|Array|AddUnique (Variables|/Script/RocketRoyal.PersistentGameInstance|GetLobbyCharacters _asbp_persistent_game_instance) _returnvalue)
  (Default|CreateTeamSelector _returnvalue)
  (return false))