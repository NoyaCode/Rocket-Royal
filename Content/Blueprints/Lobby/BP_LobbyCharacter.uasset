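; BP_LobbyCharacter is the lobby character that gives each player team selection and ready-up controls.
; CreateTeamSelector spawns a BP_TeamSelector widget for the player controller matching its Index and registers it in BP_GameModeLobby's TeamSelectors list.
; SelectTeam and GetReady input presses are forwarded to that widget.
; SetMeshPlayer swaps one mesh material slot to show whether the team is Blue or not.
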(event Custom|CreateTeamSelector
  (bind _index (Variables|Default|Getindex))
  (bind _asbp_game_mode_lobby (Utilities|Casting|CastToBP_GameModeLobby (Game|GetGameMode)))
  (bind _returnvalue (UserInterface|CreateWidget "/Game/Blueprints/Lobby/BP_TeamSelector.BP_TeamSelector_C" (Class|GameplayStatics|GetPlayerControllerfromID _index) _index))
  (UserInterface|Viewport|AddtoViewport _returnvalue 0)
  (Utilities|Array|AddUnique (Variables|/Game/Blueprints/Lobby/BP_GameModeLobby.BP_GameModeLobby_C|GetteamSelectors _asbp_game_mode_lobby) _returnvalue)
  (Variables|Default|SetTeamSelector _returnvalue))

(event EventSetMeshPlayer
  (if (Utilities|Enum|Equal(Enum) (Class|LobbyCharacter|GetTeam) (Variables|Default|GetBlue))
    (Variables|Default|SetTeamColor 0)
    (else
      (Variables|Default|SetTeamColor 1)))
  (Rendering|Material|SetMaterial (Variables|Character|GetMesh) 3 (Utilities|Select :Index (Variables|Default|GetTeamColor) :Option%200 "/Game/ImportedPack/Characters/Materials/Material_Instances/Mi_T_03_4.Mi_T_03_4" :Option%201 "/Game/ImportedPack/Characters/Materials/Material_Instances/Mi_T_03_5.Mi_T_03_5")))

(event Input|ActionEvents|InputActionSelectTeam
  (params (Key :type Key%20Structure :default "None"))
  (:Pressed
    (Default|CalledClickTeam (Variables|Default|GetTeamSelector))))

(event Input|ActionEvents|InputActionGetReady
  (params (Key :type Key%20Structure :default "None"))
  (:Pressed
    (Default|CalledClickReady (Variables|Default|GetTeamSelector))))

(fn ConstructionScript)