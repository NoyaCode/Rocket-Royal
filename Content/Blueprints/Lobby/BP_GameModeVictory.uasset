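; Victory lobby game mode that displays the winning team's characters after a match.
; On BeginPlay it adds the victory screen widget, then has the persistent game instance update team sizes and report whether blue or red won.
; It spawns team-assigned victory characters at BP_PlaceHolderPlayer markers whose Index equals the winning team's size, or also at Solo-flagged markers for a team of one.
; Spawns take only the marker's location.
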(event EventBeginPlay
  (bind _returnvalue (UserInterface|CreateWidget "/Game/Blueprints/Lobby/BP_VictoryScreenWidget.BP_VictoryScreenWidget_C" (Game|GetPlayerController 0)))
  (bind _output_get (Variables|Default|SetWidgetVictory _returnvalue))
  (UserInterface|Viewport|AddtoViewport _output_get 0)
  (bind _asbp_persistent_game_instance (Utilities|Casting|CastToBP_PersistentGameInstance (Game|GetGameInstance)))
  (bind _output_get_2 (Variables|Default|SetGameInstance _asbp_persistent_game_instance))
  (Class|PersistentGameInstance|UpdateSizeTeams _output_get_2 false)
  (if (Variables|/Script/RocketRoyal.PersistentGameInstance|GetWinningTeamBlue _output_get_2)
    (CallFunction|SpawnActors (Variables|/Script/RocketRoyal.PersistentGameInstance|GetsizeTeamBlue (Variables|Default|GetGameInstance)) true)
    (else
      (CallFunction|SpawnActors (Variables|/Script/RocketRoyal.PersistentGameInstance|GetsizeTeamRed (Variables|Default|GetGameInstance)) false))))

(event EventTick
  (params (DeltaSeconds :type Float%20%28single-precision%29)))

(fn ConstructionScript)

(fn SpawnActors
  (params (InInt :type Integer) (IsTeamBlue :type Boolean))
  (bind _outactors (Actor|GetAllActorsOfClass "/Game/Blueprints/Lobby/BP_PlaceHolderPlayer.BP_PlaceHolderPlayer_C"))
  (for _array_element _outactors
    (if (== (Variables|/Game/Blueprints/Lobby/BP_PlaceHolderPlayer.BP_PlaceHolderPlayer_C|Getindex _array_element) InInt)
      (bind _returnvalue (Game|SpawnActorfromClass "/Game/Blueprints/Lobby/BP_VictoryCharacter.BP_VictoryCharacter_C" (Math|Conversions|ToTransform(Vector) (Transformation|GetActorLocation _array_element)) "Undefined" 0 0 :!label _label))
      (Default|SetTeam _returnvalue IsTeamBlue)
      (elif (and (== InInt 1) (Variables|/Game/Blueprints/Lobby/BP_PlaceHolderPlayer.BP_PlaceHolderPlayer_C|GetSolo _array_element))
        (goto _label)))))